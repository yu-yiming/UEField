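; MotarEnemy is an enemy actor that periodically fires Projectile_A from its own location.
; Tick increments a counter by one each frame, so the firing rate follows frame rate rather than elapsed seconds.
; When the counter exceeds TimeInterval, it resets and spawns the projectile with a random whole-degree yaw within a quarter-turn arc, without targeting anything.
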(event `self.ReceiveTick`
  (params (DeltaSeconds :type "Float (single-precision)"))
  (bind _timedelta (`self.TimeDelta`))
  (`/Engine/EditorBlueprintResources/StandardMacros.IncrementFloat` _timedelta
    (:`  `
      (if (> _timedelta (`self.TimeInterval`))
        (set `self.TimeDelta` 0.0)
        (`|SpawnActorFromClass` "/Game/LevelDesign/Blueprints/Projectile_A.Projectile_A_C" (`KismetMathLibrary.MakeTransform` (`self.K2_GetActorLocation`) (`KismetMathLibrary.MakeRotator` 0.0 0.0 (`KismetMathLibrary.Conv_IntToDouble` (`KismetMathLibrary.RandomIntegerInRange` -90)))) "Undefined" "OverrideRootScale" null null)))))

(fn `UserConstructionScript`)