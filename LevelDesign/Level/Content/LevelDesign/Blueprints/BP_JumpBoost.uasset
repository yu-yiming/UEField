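; BP_JumpBoost is a pickup that temporarily raises an EpicCharacter's jump velocity.
; On overlap it applies the boost, plays a sound, toggles its visual, disables collision and brightens the HUD indicator through ThirdPersonGameMode.
; A single cooldown delay serves as both boost duration and respawn timer.
; Afterwards it restores the pickup, dims the indicator and resets jump velocity to a hard-coded default.
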(event `self.Collision.OnComponentBeginOverlap`
  (params (OverlappedComponent :type "PrimitiveComponent Object Reference") (OtherActor :type "Actor Object Reference") (OtherComp :type "PrimitiveComponent Object Reference") (OtherBodyIndex :type Integer) (bFromSweep :type Boolean) (SweepResult :type "HitResult Structure (by ref)"))
  (bind _asepic_character (cast `/Game/LevelDesign/Blueprints/EpicCharacter` OtherActor))
  (bind _charactermovement (`Character.CharacterMovement` _asepic_character))
  (set `CharacterMovementComponent.JumpZVelocity` (`self.JumpVelocity`) _charactermovement)
  (`SceneComponent.ToggleVisibility` (`self.Powerup`) false)
  (`PrimitiveComponent.SetCollisionEnabled` (`self.Collision`) "NoCollision")
  (`GameplayStatics.PlaySoundAtLocation` "/Game/LevelDesign/Audio/SFX_jump_boost.SFX_jump_boost" (`self.K2_GetActorLocation`) (struct) 1.0 1.0 0.0 null null null)
  (bind _asthird_person_game_mode (cast `/Game/LevelDesign/Blueprints/ThirdPersonGameMode` (`GameplayStatics.GetGameMode`)))
  (bind _t_jumpboost (`/Game/LevelDesign/Widgets/W_HUD.T_jumpBoost` (`/Game/LevelDesign/Blueprints/ThirdPersonGameMode.W_HUD_ref` _asthird_person_game_mode)))
  (`Image.SetColorAndOpacity` _t_jumpboost (struct :`R` 1.0 :`G` 1.0 :`B` 1.0 :`A` 1.0))
  (`KismetSystemLibrary.Delay` (`self.CoolDownTime`))
  (`SceneComponent.ToggleVisibility` (`self.Powerup`) false)
  (`PrimitiveComponent.SetCollisionEnabled` (`self.Collision`) "QueryAndPhysics")
  (`Image.SetColorAndOpacity` _t_jumpboost (struct :`R` 1.0 :`G` 1.0 :`B` 1.0 :`A` 0.3))
  (`/Engine/EditorBlueprintResources/StandardMacros.IsValid` _asepic_character
    (:`Is Valid`
      (set `CharacterMovementComponent.JumpZVelocity` 600.0 _charactermovement))))

(fn `UserConstructionScript`)