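; Bomber enemy that roams the navmesh until the player comes within its alert radius, then turns into a projectile.
; Tick checks 2D distance in the default state; Roam moves to random points, resetting state after a delay.
; When alerted, it spawns Projectile_B and smoke and destroys itself, with a delayed respawn wired afterward; a hardcoded true branch bypasses Chase.
; Hits damage a non-invincible EpicCharacter; FaceAt is an empty stub.
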(event `self.ReceiveTick`
  (params (DeltaSeconds :type "Float (single-precision)"))
  (bind _returnvalue (`self.K2_GetActorLocation`))
  (switch `/Game/LevelDesign/Blueprints/EnemyState` (`self.State`)
    (:`NewEnumerator0`
      (if (< (`KismetMathLibrary.Distance2D` (`KismetMathLibrary.Conv_VectorToVector2D` (`self.K2_GetActorLocation`)) (`KismetMathLibrary.Conv_VectorToVector2D` (`self.K2_GetActorLocation` (`GameplayStatics.GetPlayerCharacter` 0)))) (`self.AlertRadius`))
        (if true
          (set `self.OnTransform` false)
          (`|SpawnActorFromClass` "/Game/LevelDesign/Blueprints/Projectile_B.Projectile_B_C" (`self.GetTransform`) "Undefined" "OverrideRootScale" null null)
          (`self.K2_DestroyActor`)
          (`GameplayStatics.SpawnEmitterAtLocation` "/Game/StarterContent/Particles/P_Smoke.P_Smoke" _returnvalue)
          (`KismetSystemLibrary.Delay` 5.0)
          (`|SpawnActorFromClass` "BomberEnemy_C" (`KismetMathLibrary.Conv_VectorToTransform` _returnvalue) "Undefined" "OverrideRootScale" null null)
          (else
            (`self.Chase`)))
        (else
          (`self.Roam`))))))

(event `Roam`
  (bind (_returnvalue_x _returnvalue_y _returnvalue_z) (`KismetMathLibrary.BreakVector` (`self.K2_GetActorLocation`)))
  (bind _x (.x (`NavigationSystemV1.K2_GetRandomLocationInNavigableRadius` (`self.K2_GetActorLocation`) 1500.0 null null)))
  (bind _y (.y (`NavigationSystemV1.K2_GetRandomLocationInNavigableRadius` (`self.K2_GetActorLocation`) 1500.0 null null)))
  (set `self.State` "NewEnumerator1")
  (set `self.IsRoaming` true)
  (`self.FaceAt` (`KismetMathLibrary.MakeVector` _x _y _returnvalue_z))
  (`AIBlueprintHelperLibrary.SimpleMoveToLocation` (`self.GetController` self) (`KismetMathLibrary.MakeVector` _x _y))
  (`KismetSystemLibrary.Delay` 1.0)
  (set `self.State` "NewEnumerator0" :!label _label)
  (set `self.IsRoaming` false))

(event `Chase`
  (bind _returnvalue (`GameplayStatics.GetPlayerCharacter` 0))
  (bind (_returnvalue_x _returnvalue_y _returnvalue_z) (`KismetMathLibrary.BreakVector` (`self.K2_GetActorLocation`)))
  (set `self.State` "NewEnumerator2")
  (`self.FaceAt` (`KismetMathLibrary.MakeVector` (.x (`self.K2_GetActorLocation` _returnvalue)) (.y (`self.K2_GetActorLocation` _returnvalue)) _returnvalue_z))
  (`AIBlueprintHelperLibrary.SimpleMoveToActor` (`AIBlueprintHelperLibrary.GetAIController` self) _returnvalue)
  (`KismetSystemLibrary.Delay` 1.0)
  (goto _label))

(event `self.ReceiveHit`
  (params (MyComp :type "PrimitiveComponent Object Reference") (Other :type "Actor Object Reference") (OtherComp :type "PrimitiveComponent Object Reference") (bSelfMoved :type Boolean) (HitLocation :type "Vector Structure") (HitNormal :type "Vector Structure") (NormalImpulse :type "Vector Structure") (Hit :type "HitResult Structure (by ref)"))
  (bind _asepic_character (cast `/Game/LevelDesign/Blueprints/EpicCharacter` Other))
  (if (not (`/Game/LevelDesign/Blueprints/EpicCharacter.Invincible` _asepic_character))
    (`GameplayStatics.ApplyDamage` _asepic_character 1.0)))

(fn `FaceAt`
  (params (Target :type "Vector Structure")))

(fn `UserConstructionScript`)