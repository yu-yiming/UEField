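; BP_HealthPack is a health pickup that respawns a minute after use.
; When an EpicCharacter overlaps its collision, it increments player health, hides the powerup, disables collision and plays a gem sound.
; It then refreshes the lives display through the HUD reference on ThirdPersonGameMode.
; After a delay it toggles visibility back and re-enables collision, a step reached only if the game mode cast succeeds.
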(event `self.Collision.OnComponentBeginOverlap`
  (params (OverlappedComponent :type "PrimitiveComponent Object Reference") (OtherActor :type "Actor Object Reference") (OtherComp :type "PrimitiveComponent Object Reference") (OtherBodyIndex :type Integer) (bFromSweep :type Boolean) (SweepResult :type "HitResult Structure (by ref)"))
  (bind _asepic_character (cast `/Game/LevelDesign/Blueprints/EpicCharacter` OtherActor))
  (`/Engine/EditorBlueprintResources/StandardMacros.IncrementInt` (`/Game/LevelDesign/Blueprints/EpicCharacter.PlayerHealth` _asepic_character)
    (:`  `
      (`SceneComponent.ToggleVisibility` (`self.Powerup`) false)
      (`PrimitiveComponent.SetCollisionEnabled` (`self.Collision`) "NoCollision")
      (`GameplayStatics.PlaySoundAtLocation` "/Game/LevelDesign/Audio/SFX_gem.SFX_gem" (`self.K2_GetActorLocation`) (struct) 1.0 1.0 0.0 null null null)
      (bind _asthird_person_game_mode (cast `/Game/LevelDesign/Blueprints/ThirdPersonGameMode` (`GameplayStatics.GetGameMode`)))
      (`/Game/LevelDesign/Widgets/W_HUD.updateLives` (`/Game/LevelDesign/Blueprints/ThirdPersonGameMode.W_HUD_ref` _asthird_person_game_mode) _asepic_character)
      (`KismetSystemLibrary.Delay` 60.0)
      (`SceneComponent.ToggleVisibility` (`self.Powerup`) false)
      (`PrimitiveComponent.SetCollisionEnabled` (`self.Collision`) "QueryAndPhysics"))))

(fn `UserConstructionScript`)