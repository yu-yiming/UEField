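; Grenade-like explosive projectile that damages the player's EpicCharacter on contact and through a delayed blast.
; A direct hit applies minor damage unless the character is invincible.
; When projectile movement stops, it halts rotation, enables physics, waits briefly, then explodes with sound, particles and a radial impulse.
; Radial damage fires only if player 0 is vulnerable and within range, then the actor destroys itself.
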(event `self.ProjectileMovement.OnProjectileStop`
  (params (ImpactResult :type "HitResult Structure (by ref)"))
  (bind _returnvalue (`GameplayStatics.GetPlayerCharacter` 0))
  (bind _returnvalue_2 (`self.K2_GetActorLocation`))
  (bind _returnvalue_3 (`self.K2_GetActorLocation`))
  (bind _explosionradius (`self.ExplosionRadius`))
  (set `RotatingMovementComponent.RotationRate` (struct) (`self.RotatingMovement`))
  (`PrimitiveComponent.SetSimulatePhysics` (`self.Collision`) true)
  (`KismetSystemLibrary.Delay` 3.0)
  (`GameplayStatics.PlaySoundAtLocation` "/Game/StarterContent/Audio/Explosion01.Explosion01" _returnvalue_2 (struct) 1.0 1.0 0.0 null null null)
  (`GameplayStatics.SpawnEmitterAtLocation` "/Game/StarterContent/Particles/P_Explosion.P_Explosion" _returnvalue_2)
  (`RadialForceComponent.FireImpulse` (`self.RadialForce`))
  (bind _asepic_character (cast `/Game/LevelDesign/Blueprints/EpicCharacter` _returnvalue))
  (if (and (not (`/Game/LevelDesign/Blueprints/EpicCharacter.Invincible` _asepic_character)) (< (`KismetMathLibrary.Vector_Distance` _returnvalue_3 (`self.K2_GetActorLocation` _returnvalue)) _explosionradius))
    (`GameplayStatics.ApplyRadialDamage` :`BaseDamage` (`self.ExplosionPower`) :`Origin` _returnvalue_3 :`DamageRadius` _explosionradius :`DamageTypeClass` "/Script/Engine.DamageType" :`DamageCauser` self :`InstigatedByController` null))
  (`self.K2_DestroyActor`))

(event `self.Collision.OnComponentHit`
  (params (HitComponent :type "PrimitiveComponent Object Reference") (OtherActor :type "Actor Object Reference") (OtherComp :type "PrimitiveComponent Object Reference") (NormalImpulse :type "Vector Structure") (Hit :type "HitResult Structure (by ref)"))
  (bind _asepic_character (cast `/Game/LevelDesign/Blueprints/EpicCharacter` OtherActor))
  (if (not (`/Game/LevelDesign/Blueprints/EpicCharacter.Invincible` _asepic_character))
    (`GameplayStatics.ApplyDamage` _asepic_character 1.0 null self "/Script/Engine.DamageType")))

(event `self.ProjectileMovement.OnProjectileBounce`
  (params (ImpactResult :type "HitResult Structure (by ref)") (ImpactVelocity :type "Vector Structure (by ref)")))

(fn `UserConstructionScript`)