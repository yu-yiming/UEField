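; Projectile_B is a timed explosive actor that detonates after a countdown and then destroys itself.
; BeginPlay sizes the RadialForce component to the explosion radius, waits, then plays explosion sound and particles and fires a physics impulse.
; Radial damage is applied only when the player character is within the radius, so other actors take none unless the player is also in range.
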(event `self.ReceiveBeginPlay`
  (bind _returnvalue (`self.K2_GetActorLocation`))
  (bind _returnvalue_2 (`self.K2_GetActorLocation`))
  (bind _explosionradius (`self.ExplosionRadius`))
  (set `RadialForceComponent.Radius` (`self.ExplosionRadius`) (`self.RadialForce`))
  (`KismetSystemLibrary.Delay` (`self.CountDown`))
  (`GameplayStatics.PlaySoundAtLocation` "/Game/StarterContent/Audio/Explosion01.Explosion01" _returnvalue (struct) 1.0 1.0 0.0 null null null)
  (`GameplayStatics.SpawnEmitterAtLocation` "/Game/StarterContent/Particles/P_Explosion.P_Explosion" _returnvalue)
  (`RadialForceComponent.FireImpulse` (`self.RadialForce`))
  (if (< (`KismetMathLibrary.Vector_Distance` _returnvalue_2 (`self.K2_GetActorLocation` (`GameplayStatics.GetPlayerCharacter` 0))) _explosionradius)
    (`GameplayStatics.ApplyRadialDamage` :`BaseDamage` (`self.ExplosionPower`) :`Origin` _returnvalue_2 :`DamageRadius` _explosionradius :`DamageTypeClass` "/Script/Engine.DamageType" :`DamageCauser` self :`InstigatedByController` null))
  (`self.K2_DestroyActor`))

(fn `UserConstructionScript`)