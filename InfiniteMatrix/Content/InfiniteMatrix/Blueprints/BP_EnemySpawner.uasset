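; Enemy spawner that keeps a population of BP_Enemy actors ahead of the player along +X.
; Each tick, while the enemy count is at most MaxEnemy, it decrements CountDown or, once that runs out, spawns a scaled-down enemy at a random offset from the player.
; Spawned enemies receive a spawner reference; DestroyEnemy removes one and lowers the count.
; CoolDown restarts the tick-based delay but is not called within this Blueprint.
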(event `self.ReceiveTick`
  (params (DeltaSeconds :type "Float (single-precision)"))
  (bind _countdown (`self.CountDown`))
  (if (<= (`self.Enemy`) (`self.MaxEnemy`))
    (if (> _countdown 0)
      (`/Engine/EditorBlueprintResources/StandardMacros.DecrementInt` _countdown)
      (else
        (`self.SpawnEnemy`)))))

(fn `CoolDown`
  (set `self.CountDown` 1000))

(fn `DestroyEnemy`
  (params (Enemy :type "/Game/InfiniteMatrix/Blueprints/BP_Enemy Object Reference"))
  (`self.K2_DestroyActor` Enemy)
  (`/Engine/EditorBlueprintResources/StandardMacros.DecrementInt` (`self.Enemy`)))

(fn `SpawnEnemy`
  (bind (_returnvalue_x _returnvalue_y _returnvalue_z) (`KismetMathLibrary.BreakVector` (`self.K2_GetActorLocation` (`GameplayStatics.GetPlayerPawn` 0))))
  (bind _returnvalue (`|SpawnActorFromClass` "/Game/InfiniteMatrix/Blueprints/BP_Enemy.BP_Enemy_C" (`KismetMathLibrary.MakeTransform` (`KismetMathLibrary.MakeVector` (+ _returnvalue_x (`KismetMathLibrary.RandomFloatInRange` 2000.0 5000.0)) (+ _returnvalue_y (`KismetMathLibrary.RandomFloatInRange` -200.0 200.0)) (+ _returnvalue_z (`KismetMathLibrary.RandomFloatInRange` -150.0 150.0))) (struct) (0.2 0.2 0.2)) "Undefined" "OverrideRootScale" null null))
  (set `/Game/InfiniteMatrix/Blueprints/BP_Enemy.EnemySpawner` self _returnvalue)
  (`/Engine/EditorBlueprintResources/StandardMacros.IncrementInt` (`self.Enemy`)))

(fn `UserConstructionScript`)