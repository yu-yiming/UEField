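; BP_ItemSpawner spawns BP_Item pickups ahead of the player, keeping at most one pending item at a time.
; Each tick, when no valid NextItem exists, a random roll may trigger SpawnItem.
; SpawnItem places the item at a random forward offset along X from the player pawn, with Y and Z jitter, and assigns a random mesh from MeshList.
; The new item receives a reference back to the spawner.
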(event `self.ReceiveBeginPlay`)

(event `self.ReceiveTick`
  (params (DeltaSeconds :type "Float (single-precision)"))
  (if (and (not (`KismetSystemLibrary.IsValid` (`self.NextItem`))) (> (`KismetMathLibrary.RandomFloat`) 0.85))
    (`self.SpawnItem`)))

(fn `SpawnItem`
  (bind (_returnvalue_x _returnvalue_y _returnvalue_z) (`KismetMathLibrary.BreakVector` (`self.K2_GetActorLocation` (`GameplayStatics.GetPlayerPawn` 0))))
  (bind _returnvalue (`|SpawnActorFromClass` "/Game/InfiniteMatrix/Blueprints/BP_Item.BP_Item_C" (`KismetMathLibrary.MakeTransform` (`KismetMathLibrary.MakeVector` (+ _returnvalue_x (`KismetMathLibrary.RandomFloatInRange` 2000.0 5000.0)) (+ _returnvalue_y (`KismetMathLibrary.RandomFloatInRange` -200.0 200.0)) (+ _returnvalue_z (`KismetMathLibrary.RandomFloatInRange` -150.0 150.0)))) "Undefined" "OverrideRootScale" null null))
  (`|ExecutionSequence`
    (:`then_0`
      ;[1 1 1] Set random mesh
      (bind _output_get (set `self.NextItemID` (`KismetMathLibrary.RandomInteger` 4)))
      (`StaticMeshComponent.SetStaticMesh` (`/Game/InfiniteMatrix/Blueprints/BP_Item.ItemMesh` _returnvalue) (`|GetArrayItem` (`self.MeshList`) _output_get)))
    (:`then_1`
      (set `/Game/InfiniteMatrix/Blueprints/BP_Item.ItemSpawner` self _returnvalue)
      (set `self.NextItem` _returnvalue))))

(fn `UserConstructionScript`)