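; BP_Item is a collectible pickup that spins in place and destroys itself once the player pawn passes it along X.
; When its mesh hits BP_Player, it applies an effect, refreshes the player's info and destroys itself.
; EffectOn picks heart, coin score, projectile or bomb by reading ItemSpawner's NextItemID at hit time, rather than an ID stored on the item.
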(event `self.ReceiveTick`
  (params (DeltaSeconds :type "Float (single-precision)"))
  (bind _returnvalue_x (`KismetMathLibrary.BreakVector` (`self.K2_GetActorLocation`)))
  (bind _returnvalue_x_2 (`KismetMathLibrary.BreakVector` (`self.K2_GetActorLocation` (`GameplayStatics.GetPlayerPawn` 0))))
  ;[1 1 1] Generate, rotate, and destroy item
  (`SceneComponent.K2_AddLocalRotation` (`self.ItemMesh`) (`KismetMathLibrary.MakeRotator` 0.0 0.0 (* DeltaSeconds (`self.ItemRotateSpeed`))) false false)
  (if (> _returnvalue_x_2 (+ _returnvalue_x 100.0))
    (`self.K2_DestroyActor`)))

(event `self.ItemMesh.OnComponentHit`
  (params (HitComponent :type "PrimitiveComponent Object Reference") (OtherActor :type "Actor Object Reference") (OtherComp :type "PrimitiveComponent Object Reference") (NormalImpulse :type "Vector Structure") (Hit :type "HitResult Structure (by ref)"))
  ;[1 1 1] Collect items on hit
  (bind _asbp_player (cast `/Game/InfiniteMatrix/Blueprints/BP_Player` OtherActor))
  (`self.EffectOn` _asbp_player)
  (`/Game/InfiniteMatrix/Blueprints/BP_Player.UpdatePlayerInfo` _asbp_player)
  (`self.K2_DestroyActor`))

(fn `EffectOn`
  (params (Player :type "/Game/InfiniteMatrix/Blueprints/BP_Player Object Reference"))
  (bind _nextitemid (`/Game/InfiniteMatrix/Blueprints/BP_ItemSpawner.NextItemID` (`self.ItemSpawner`)))
  ;[1 1 1] Heart
  (if (== _nextitemid 0)
    (`/Game/InfiniteMatrix/Blueprints/BP_Player.IncHealth` Player)
    (else
      ;[1 1 1] Coin
      (if (== _nextitemid 1)
        (set `/Game/InfiniteMatrix/Blueprints/BP_Player.Score` (+ (`/Game/InfiniteMatrix/Blueprints/BP_Player.Score` Player) 5) Player)
        (else
          ;[1 1 1] Projectile
          (if (== _nextitemid 2)
            (`/Game/InfiniteMatrix/Blueprints/BP_Player.IncProjectile` Player)
            (else
              ;[1 1 1] Bomb
              (if (== _nextitemid 3)
                (set `/Game/InfiniteMatrix/Blueprints/BP_Player.HasBomb` true Player)))))))))

(fn `UserConstructionScript`)