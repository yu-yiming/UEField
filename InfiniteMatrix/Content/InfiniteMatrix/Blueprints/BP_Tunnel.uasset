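; BP_Tunnel is a tunnel segment with a spinning holed wall that the player must pass through.
; RandomizeWall picks a hole mesh and random roll, and Tick spins it faster as DifficultyFactor rises.
; Hitting the wall costs health once via the player's JustHit flag.
; Trigger overlap spawns the next segment through TunnelSpawner and destroys this one; end overlap awards difficulty-scaled score if unhit, then clears JustHit.
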(event `self.ReceiveBeginPlay`)

(event `self.ReceiveTick`
  (params (DeltaSeconds :type "Float (single-precision)"))
  (bind _wallmesh (`self.WallMesh`))
  ;[1 1 1] Rotate walls and items
  (bind _asbp_player (cast `/Game/InfiniteMatrix/Blueprints/BP_Player` (`GameplayStatics.GetPlayerPawn` 0)))
  (`/Engine/EditorBlueprintResources/StandardMacros.IsValid` _wallmesh
    (:`Is Valid`
      (`SceneComponent.K2_AddLocalRotation` _wallmesh (`KismetMathLibrary.MakeRotator` (* DeltaSeconds (+ (`KismetMathLibrary.Conv_IntToDouble` (/ (`/Game/InfiniteMatrix/Blueprints/BP_Player.DifficultyFactor` _asbp_player) 10)) (`self.WallRotateSpeed`)))) false false))))

(event `self.TriggerZone.OnComponentBeginOverlap`
  (params (OverlappedComponent :type "PrimitiveComponent Object Reference") (OtherActor :type "Actor Object Reference") (OtherComp :type "PrimitiveComponent Object Reference") (OtherBodyIndex :type Integer) (bFromSweep :type Boolean) (SweepResult :type "HitResult Structure (by ref)"))
  ;[1 1 1] Generate walls
  (cast `/Game/InfiniteMatrix/Blueprints/BP_Player` OtherActor)
  (`/Game/InfiniteMatrix/Blueprints/BP_TunnelSpawner.SpawnTunnelAtSpawnPoint` (`self.TunnelSpawner`))
  (`self.K2_DestroyActor`))

(event `self.WallMesh.OnComponentHit`
  (params (HitComponent :type "PrimitiveComponent Object Reference") (OtherActor :type "Actor Object Reference") (OtherComp :type "PrimitiveComponent Object Reference") (NormalImpulse :type "Vector Structure") (Hit :type "HitResult Structure (by ref)"))
  ;[1 1 1] On hitting the wall
  (bind _asbp_player (cast `/Game/InfiniteMatrix/Blueprints/BP_Player` OtherActor))
  (if (not (`/Game/InfiniteMatrix/Blueprints/BP_Player.JustHit` _asbp_player))
    (set `/Game/InfiniteMatrix/Blueprints/BP_Player.JustHit` true _asbp_player)
    (`/Game/InfiniteMatrix/Blueprints/BP_Player.DecHealth` _asbp_player)
    (`/Game/InfiniteMatrix/Blueprints/BP_Player.UpdatePlayerInfo` _asbp_player)))

(event `self.TriggerZone.OnComponentEndOverlap`
  (params (OverlappedComponent :type "PrimitiveComponent Object Reference") (OtherActor :type "Actor Object Reference") (OtherComp :type "PrimitiveComponent Object Reference") (OtherBodyIndex :type Integer))
  ;[1 1 1] Update player info
  (bind _asbp_player (cast `/Game/InfiniteMatrix/Blueprints/BP_Player` OtherActor))
  (if (not (`/Game/InfiniteMatrix/Blueprints/BP_Player.JustHit` _asbp_player))
    (`/Game/InfiniteMatrix/Blueprints/BP_Player.IncScore` _asbp_player (`KismetMathLibrary.Max` (/ (`/Game/InfiniteMatrix/Blueprints/BP_Player.DifficultyFactor` _asbp_player) 10) 1)))
  (`/Game/InfiniteMatrix/Blueprints/BP_Player.UpdatePlayerInfo` _asbp_player)
  (set `/Game/InfiniteMatrix/Blueprints/BP_Player.JustHit` false _asbp_player))

(fn `RandomizeWall`
  (`StaticMeshComponent.SetStaticMesh` (`self.WallMesh`) (select `int` (`KismetMathLibrary.RandomInteger` 3) :`0` "/Game/InfiniteMatrix/Meshes/SM_Hole_01.SM_Hole_01" :`1` "/Game/InfiniteMatrix/Meshes/SM_Hole_02.SM_Hole_02" :`2` "/Game/InfiniteMatrix/Meshes/SM_Hole_03.SM_Hole_03" :`3` "/Game/InfiniteMatrix/Meshes/SM_Hole_04.SM_Hole_04" :!type "StaticMesh Object Reference"))
  (`SceneComponent.K2_AddLocalRotation` (`self.WallMesh`) (`KismetMathLibrary.MakeRotator` (`KismetMathLibrary.RandomFloatInRange` 0.0 360.0)) false false))

(fn `UserConstructionScript`)