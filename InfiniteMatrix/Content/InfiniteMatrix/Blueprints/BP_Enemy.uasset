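; Enemy actor that damages the player on contact and can be destroyed by projectiles.
; A mesh hit on the player lowers their health and refreshes player info, while a projectile overlap only kills the enemy, both routed through the EnemySpawner's DestroyEnemy.
; Tick removes the enemy once the player moves past it along X, decrementing the spawner's enemy count directly.
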(event `self.ReceiveBeginPlay`)

(event `self.ReceiveTick`
  (params (DeltaSeconds :type "Float (single-precision)"))
  (bind _returnvalue_x (`KismetMathLibrary.BreakVector` (`self.K2_GetActorLocation`)))
  (bind _returnvalue_x_2 (`KismetMathLibrary.BreakVector` (`self.K2_GetActorLocation` (`GameplayStatics.GetPlayerPawn` 0))))
  (if (> _returnvalue_x_2 (+ _returnvalue_x 100.0))
    (`self.K2_DestroyActor`)
    (`/Engine/EditorBlueprintResources/StandardMacros.DecrementInt` (`/Game/InfiniteMatrix/Blueprints/BP_EnemySpawner.Enemy` (`self.EnemySpawner`)))))

(event `self.EnemyMesh.OnComponentHit`
  (params (HitComponent :type "PrimitiveComponent Object Reference") (OtherActor :type "Actor Object Reference") (OtherComp :type "PrimitiveComponent Object Reference") (NormalImpulse :type "Vector Structure") (Hit :type "HitResult Structure (by ref)"))
  (bind _asbp_player (cast `/Game/InfiniteMatrix/Blueprints/BP_Player` OtherActor))
  (`/Game/InfiniteMatrix/Blueprints/BP_Player.DecHealth` _asbp_player)
  (`/Game/InfiniteMatrix/Blueprints/BP_Player.UpdatePlayerInfo` _asbp_player)
  (`/Game/InfiniteMatrix/Blueprints/BP_EnemySpawner.DestroyEnemy` (`self.EnemySpawner`) self))

(event `self.EnemyMesh.OnComponentBeginOverlap`
  (params (OverlappedComponent :type "PrimitiveComponent Object Reference") (OtherActor :type "Actor Object Reference") (OtherComp :type "PrimitiveComponent Object Reference") (OtherBodyIndex :type Integer) (bFromSweep :type Boolean) (SweepResult :type "HitResult Structure (by ref)"))
  (cast `/Game/InfiniteMatrix/Blueprints/BP_Projectile` OtherActor)
  (`/Game/InfiniteMatrix/Blueprints/BP_EnemySpawner.DestroyEnemy` (`self.EnemySpawner`) self))

(fn `UserConstructionScript`)