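; BP_Projectile is a projectile that kills enemies and earns score for the Source that owns it.
; Each tick it sweeps along world X at its own forward speed plus that of Source.
; When its mesh hits a BP_Enemy, it has that enemy's spawner destroy it and increments the Source's score.
; The projectile destroys itself on any mesh hit.
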(event `self.ReceiveTick`
  (params (DeltaSeconds :type "Float (single-precision)"))
  (`self.K2_AddActorWorldOffset` (`KismetMathLibrary.MakeVector` (* DeltaSeconds (+ (`/Game/InfiniteMatrix/Blueprints/BP_Player.ForwardSpeed` (`self.Source`)) (`self.ForwardSpeed`)))) true))

(event `self.ProjectileMesh.OnComponentHit`
  (params (HitComponent :type "PrimitiveComponent Object Reference") (OtherActor :type "Actor Object Reference") (OtherComp :type "PrimitiveComponent Object Reference") (NormalImpulse :type "Vector Structure") (Hit :type "HitResult Structure (by ref)"))
  (`|ExecutionSequence`
    (:`then_0`
      (bind _asbp_enemy (cast `/Game/InfiniteMatrix/Blueprints/BP_Enemy` OtherActor))
      (`/Game/InfiniteMatrix/Blueprints/BP_EnemySpawner.DestroyEnemy` (`/Game/InfiniteMatrix/Blueprints/BP_Enemy.EnemySpawner` _asbp_enemy) _asbp_enemy)
      (`/Game/InfiniteMatrix/Blueprints/BP_Player.IncScore` (`self.Source`) 5))
    (:`then_1`
      (`self.K2_DestroyActor`))))

(fn `OnHit`
  (params (SelfActor :type "Actor Object Reference") (OtherActor :type "Actor Object Reference") (NormalImpulse :type "Vector Structure") (Hit :type "HitResult Structure (by ref)"))
  (`self.K2_DestroyActor` SelfActor)
  (return))

(fn `UserConstructionScript`)